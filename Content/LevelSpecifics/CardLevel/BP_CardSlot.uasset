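; BP_CardSlot is a slot in the card level where grabbable cards stack, and a slot flagged as winning completes the level.
; On overlap it plays a placement sound and counts the BP_Cards, cached at BeginPlay, whose InterpFollower is using this slot.
; The incoming object's InterpFollower then follows the slot, with height offset by that count.
; A high enough count on a winning slot calls WinLevel on GamePlayerController after a short timer.
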(event OnComponentBeginOverlap(CardCollision)
  (params (OverlappedComponent :type Primitive%20Component%20Object%20Reference) (OtherActor :type Actor%20Object%20Reference) (OtherComp :type Primitive%20Component%20Object%20Reference) (OtherBodyIndex :type Integer) (bFromSweep :type Boolean) (SweepResult :type Hit%20Result%20Structure%20%28by%20ref%29))
  (bind _returnvalue (Actor|GetComponentbyClass OtherActor "/Script/GameOff2022.InterpFollower"))
  (if (Actor|ActorHasTag OtherActor "Grabbable")
    (Audio|PlaySoundatLocation "/Game/Common/Assets/Sounds/Other/SC_CardPlace.SC_CardPlace" (Transformation|GetActorLocation) "0, 0, 0" 1.0 1.0 0.0 0 0 0 0)
    (Variables|Default|SetCardsInStack 0)
    (for _array_element (Variables|Default|GetCards)
      (if (== (Variables|/Script/GameOff2022.InterpFollower|GetCurrentUser (Actor|GetComponentbyClass _array_element "/Script/GameOff2022.InterpFollower")) self)
        (Math|Integer|IncrementInt (Variables|Default|GetCardsInStack))))
    (Utilities|IsValid _returnvalue
      (:Is%20Valid
        (Class|InterpFollower|StartFollowing _returnvalue (Variables|Default|GetSceneRoot) "EHS_None" self (Math|Transform|MakeTransform (Math|Vector|MakeVector 0.0 0.0 (Math|Conversions|ToFloat(Integer) (+ (Variables|Default|GetCardsInStack) 3))) "90.000000,180.000000,0.000000" "0.800000,0.800000,0.800000")))
      (:Is%20Not%20Valid
        _))
    (if (and (>= (Variables|Default|GetCardsInStack) 3) (Variables|Default|GetbWinningCardSlot))
      (Utilities|Time|SetTimerbyEvent (delegate Custom|WinGame) 0.5))))

(event Custom|WinGame
  (bind _asgame_player_controller (Utilities|Casting|CastToGamePlayerController (Game|GetPlayerController 0)))
  (Class|GamePlayerController|WinLevel _asgame_player_controller))

(event EventBeginPlay
  (bind _outactors (Actor|GetAllActorsOfClass "/Game/LevelSpecifics/CardLevel/Cards/BP_Card.BP_Card_C"))
  (Variables|Default|SetCards _outactors))

(fn ConstructionScript)