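; Lemon container for the lemon level that turns a lemon into lemonade and wins the level.
; When a Grabbable-tagged actor overlaps LemonCollision, its InterpFollower component pulls it onto the container at a small scale.
; Short chained timers then destroy that actor, reveal the lemonade mesh and call WinLevel on the GamePlayerController.
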(event OnComponentBeginOverlap(LemonCollision)
  (params (OverlappedComponent :type Primitive%20Component%20Object%20Reference) (OtherActor :type Actor%20Object%20Reference) (OtherComp :type Primitive%20Component%20Object%20Reference) (OtherBodyIndex :type Integer) (bFromSweep :type Boolean) (SweepResult :type Hit%20Result%20Structure%20%28by%20ref%29))
  (if (Actor|ActorHasTag OtherActor "Grabbable")
    (Variables|Default|SetLemon OtherActor)
    (Class|InterpFollower|StartFollowing (Actor|GetComponentbyClass OtherActor "/Script/GameOff2022.InterpFollower") (Variables|Default|GetSceneRoot) "EHS_None" self (Math|Transform|MakeTransform "1.000000,2.000000,15.000000" "0.000000,0.000000,0.000000" "0.100000,0.100000,0.100000"))
    (Utilities|Time|SetTimerbyEvent (delegate Custom|MakeLemonad) 0.5)))

(event Custom|MakeLemonad
  (Actor|DestroyActor (Variables|Default|GetLemon))
  (Rendering|SetVisibility (Variables|Default|GetLemonadeMesh) true false)
  (Utilities|Time|SetTimerbyEvent (delegate Custom|WinGame) 0.7))

(event Custom|WinGame
  (bind _asgame_player_controller (Utilities|Casting|CastToGamePlayerController (Game|GetPlayerController 0)))
  (Class|GamePlayerController|WinLevel _asgame_player_controller))

(fn ConstructionScript)