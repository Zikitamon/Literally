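; BP_Facusable is the FaceLevel target: a drifting actor that the player must keep centered in view to win.
; Its physics sphere accelerates in periodically re-randomized, vertically damped directions while the actor turns to face the player.
; Each tick, a multi-trace from the view point slowly raises Score on a hit and drains it faster otherwise.
; Score thresholds trigger WinLevel or LoseLevel on GamePlayerController and stop further scoring.
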(event Custom|ChangeForceDirection
  (bind _returnvalue (Math|Random|RandomUnitVector))
  (Variables|Default|SetForceDirection (Math|Vector|MakeVector (.x _returnvalue) (.y _returnvalue) (* (.z _returnvalue) 0.25)))
  (Utilities|Time|SetTimerbyEvent (delegate Custom|ChangeForceDirection) (Math|Random|RandomFloatinRange 0.5 3.0)))

(event EventBeginPlay
  (Variables|Default|SetScore 1e+01)
  (CallFunction|ChangeForceDirection))

(event EventTick
  (params (DeltaSeconds :type Float%20%28single-precision%29))
  (bind _returnvalue (Game|GetPlayerController 0))
  (bind (_location _rotation) (Pawn|GetPlayerViewPoint _returnvalue))
  (Physics|AddForce (Variables|Default|GetSphere) (* (Variables|Default|GetForceDirection) 1e+02) "None" true)
  (Transformation|SetActorRotation (Math|Conversions|RotationFromXVector (- (Transformation|GetActorLocation (Pawn|GetControlledPawn _returnvalue)) (Transformation|GetActorLocation))))
  (if (not (Variables|Default|GetbLevelOver))
    (bind _outhits (Collision|MultiLineTraceByChannel _location (+ _location (* (Math|Vector|GetForwardVector _rotation) 1e+04)) "TraceTypeQuery1" false (Utilities|Array|MakeArray (Pawn|GetControlledPawn _returnvalue)) "None" false))
    (Variables|Default|SetbHittingSelf false)
    (for _array_element _outhits
      (if (== self (.HitActor (Collision|BreakHitResult _array_element)))
        (Variables|Default|SetbHittingSelf true)))
    (if (Variables|Default|GetbHittingSelf)
      (Variables|Default|SetScore (+ (Variables|Default|GetScore) DeltaSeconds))
      (else
        (Variables|Default|SetScore (- (Variables|Default|GetScore) (* DeltaSeconds 3.0)))))
    (if (> (Variables|Default|GetScore) 2e+01)
      (bind _asgame_player_controller (Utilities|Casting|CastToGamePlayerController _returnvalue))
      (Class|GamePlayerController|WinLevel _asgame_player_controller)
      (Variables|Default|SetbLevelOver true :!label _label)
      (elif (<= (Variables|Default|GetScore) 0.0)
        (bind _asgame_player_controller_2 (Utilities|Casting|CastToGamePlayerController _returnvalue))
        (Class|GamePlayerController|LoseLevel _asgame_player_controller_2)
        (goto _label)))))

(fn ConstructionScript)