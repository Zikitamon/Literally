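; BP_Bull is a wandering bull enemy for the Bull level that can charge the player and make them lose the level.
; Randomized timers alternate walking in a random direction with pauses, during which it may face a nearby player and often schedule a dash.
; The dash is an upward-biased impulse toward the player, and capsule overlaps during its brief window trigger LoseLevel.
; Movement and dashing run only while InterpFollower has no current user.
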(event OnComponentBeginOverlap(Capsule)
  (params (OverlappedComponent :type Primitive%20Component%20Object%20Reference) (OtherActor :type Actor%20Object%20Reference) (OtherComp :type Primitive%20Component%20Object%20Reference) (OtherBodyIndex :type Integer) (bFromSweep :type Boolean) (SweepResult :type Hit%20Result%20Structure%20%28by%20ref%29))
  (if (Variables|Default|GetbDashing)
    (bind _aspawn (Utilities|Casting|CastToPawn OtherActor))
    (bind _asgame_player_controller (Utilities|Casting|CastToGamePlayerController (Pawn|GetController _aspawn)))
    (Class|GamePlayerController|LoseLevel _asgame_player_controller)))

(event Custom|UpdateTargetDirection
  (Variables|Default|SetbIsMoving (not (Variables|Default|GetbIsMoving)))
  (Variables|Default|SetTargetDirection (Math|Rotator|MakeRotator 0.0 0.0 (Math|Random|RandomFloatinRange -1.8e+02 1.8e+02)))
  (if (Variables|Default|GetbIsMoving)
    (Utilities|Time|SetTimerbyEvent (delegate Custom|UpdateTargetDirection) (Math|Random|RandomFloatinRange 2.0 4.0))
    (else
      (Utilities|Time|SetTimerbyEvent (delegate Custom|UpdateTargetDirection) (Math|Random|RandomFloatinRange 3.0 1e+01))
      (bind _output_get (Variables|Default|SetbShouldLookAtPlayer (and (< (Math|Random|RandomFloatinRange 0.0 1.0) 0.4) (< (Transformation|GetDistanceTo (Game|Player|GetPlayerPawn 0) self) 8e+02))))
      (if (and _output_get (< (Math|Random|RandomFloatinRange 0.0 1.0) 0.7))
        (Utilities|Time|SetTimerbyEvent (delegate Custom|Dash) 1.0)))))

(event Custom|Dash
  (if (== (Variables|/Script/GameOff2022.InterpFollower|GetCurrentUser (Variables|Default|GetInterpFollower)) 0)
    (Physics|AddImpulse (Variables|Character|GetCharacterMovement) (+ (* (Math|Vector|Normalize (- (Transformation|GetActorLocation (Game|Player|GetPlayerPawn 0)) (Transformation|GetActorLocation))) 5e+03) "0.000000,0.000000,500.000000") true)
    (Variables|Default|SetbDashing true)
    (Utilities|Time|SetTimerbyEvent (delegate Custom|ClearDashingStatus) 0.5)))

(event Custom|ClearDashingStatus
  (Variables|Default|SetbDashing false))

(event EventBeginPlay
  (Utilities|Time|SetTimerbyEvent (delegate Custom|UpdateTargetDirection) (Math|Random|RandomFloatinRange 3.0 5.0)))

(event EventTick
  (params (DeltaSeconds :type Float%20%28single-precision%29))
  (if (== (Variables|/Script/GameOff2022.InterpFollower|GetCurrentUser (Variables|Default|GetInterpFollower)) 0)
    (if (Variables|Default|GetbIsMoving)
      (Pawn|Input|AddMovementInput (Math|Vector|GetForwardVector (Variables|Default|GetTargetDirection)) 1.0 false)
      (elif (Variables|Default|GetbShouldLookAtPlayer)
        (Pawn|Input|AddMovementInput (Math|Vector|Normalize (- (Transformation|GetActorLocation (Game|Player|GetPlayerPawn 0)) (Transformation|GetActorLocation))) 0.01 false)))))

(fn ConstructionScript)