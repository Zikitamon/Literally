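; BP_HorseMouthDetector is a horse-level actor that makes the player lose the level when their view points at it.
; Each tick it runs a long multi line trace on the Visibility channel along the player's view direction, ignoring the controlled pawn.
; If any hit is this actor, it calls LoseLevel on GamePlayerController and sets LevelLost, which stops further checks.
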(event EventTick
  (params (DeltaSeconds :type Float%20%28single-precision%29))
  (bind _returnvalue (Game|GetPlayerController 0))
  (bind (_location _rotation) (Pawn|GetPlayerViewPoint _returnvalue))
  (if (not (Variables|Default|GetbLevelLost))
    (bind _outhits (Collision|MultiLineTraceByChannel _location (+ _location (* (Math|Vector|GetForwardVector _rotation) 1e+04)) "TraceTypeQuery1" false (Utilities|Array|MakeArray (Pawn|GetControlledPawn _returnvalue)) "None" false))
    (for _array_element _outhits
      (if (== self (.HitActor (Collision|BreakHitResult _array_element)))
        (bind _asgame_player_controller (Utilities|Casting|CastToGamePlayerController _returnvalue))
        (Class|GamePlayerController|LoseLevel _asgame_player_controller)
        (Variables|Default|SetbLevelLost true)))))

(fn ConstructionScript)